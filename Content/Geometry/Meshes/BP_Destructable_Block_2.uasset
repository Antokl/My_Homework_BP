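; Destructible block Blueprint that shrinks each time it is hit instead of breaking apart.
; The Hit event subtracts the Delta vector from the actor's scale, as long as the resulting X scale stays at or above Delta's X, so the block is never destroyed.
; The node setting Delta to 5% of the current scale is unconnected, so Delta keeps its default; BeginPlay's validity check leads nowhere.
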(event EventBeginPlay
  (|CallParentFunction)
  (Utilities|IsValid self))

(event Collision|EventActorBeginOverlap
  (params (OtherActor :type Actor%20Object%20Reference))
  (|CallParentFunction OtherActor) ; This node is disabled and will not be called.\nDrag off pins to build functionality.
)

(event EventTick
  (params (DeltaSeconds :type Float%20%28single-precision%29))
  (|CallParentFunction DeltaSeconds) ; This node is disabled and will not be called.\nDrag off pins to build functionality.
)

(event Collision|EventHit
  (params (MyComp :type Primitive%20Component%20Object%20Reference) (Other :type Actor%20Object%20Reference) (OtherComp :type Primitive%20Component%20Object%20Reference) (bSelfMoved :type Boolean) (HitLocation :type Vector :default "0, 0, 0") (HitNormal :type Vector :default "0, 0, 0") (NormalImpulse :type Vector :default "0, 0, 0") (Hit :type Hit%20Result%20Structure%20%28by%20ref%29))
  (bind _returnvalue (Transformation|GetActorScale3D))
  (bind _delta (Variables|Default|GetDelta))
  (bind _returnvalue_2 (- _returnvalue _delta))
  (|CallParentFunction MyComp Other OtherComp bSelfMoved HitLocation HitNormal NormalImpulse Hit)
  (if (>= (.x _returnvalue_2) (.x (Variables|Default|GetDelta)))
    (Transformation|SetActorScale3D (Math|Vector|MakeVector (.x _returnvalue_2) (.y _returnvalue_2) (.z _returnvalue_2)))))

(fn ConstructionScript
  (|CallParentFunction))